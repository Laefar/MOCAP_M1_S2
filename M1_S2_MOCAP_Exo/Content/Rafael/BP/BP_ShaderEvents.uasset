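; Event-driven actor for MetaHuman face effects: tongue soap bubbles, demon horns and head scaling.
; On BeginPlay it finds the first MetaHuman's face mesh via Manager_MetaHuman, then attaches the Niagara bubble and horn mesh to sockets.
; Events toggle bubbles, animate horn Erosion and Hot material parameters by timeline, and play or reverse a head-scale timeline.
; The head-scale write to the AnimInstance is disconnected with a broken cast, and SpawnLightBulb is empty.
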(event `self.ReceiveBeginPlay`
  (bind _skel_demonhorn (`self.Skel_DemonHorn`))
  (`|ExecutionSequence`
    (:`then_0`
      ;[0.08854 0.08854 0.08854] Get MetaHuman's Anim Instance
      (bind _returnvalue (`GameplayStatics.GetActorOfClass` "/Game/Cassandra/Manager_MetaHuman.Manager_MetaHuman_C"))
      (for _array_element (`self.K2_GetComponentsByClass` (`|GetArrayItem` (`/Game/Cassandra/Manager_MetaHuman.MetaHumans` _returnvalue)) "/Script/Engine.SkeletalMeshComponent")
        (if (and (`KismetSystemLibrary.IsValid` _array_element) (`KismetStringLibrary.Contains` (`KismetSystemLibrary.GetDisplayName` _array_element) ".Face"))
          (set `self.AnimInstance` (`SkeletalMeshComponent.GetAnimInstance` _array_element))
          (set `self.FaceMesh` _array_element))))
    (:`then_1`
      ;[0.08854 0.08854 0.08854] Attach Soap Bubble FX to MetaHuman
      (`SceneComponent.K2_AttachToComponent` (`self.Niagara_SoapBubble`) (`self.FaceMesh`) "FACIAL_C_TongueUpper1" "SnapToTarget" "SnapToTarget" "KeepWorld" true))
    (:`then_2`
      ;[0.08854 0.08854 0.08854] Attach Horn on MetaHuman + Set Dynamic Material
      (`SceneComponent.K2_AttachToComponent` _skel_demonhorn (`self.FaceMesh`) "head" "KeepRelative" "KeepRelative" "SnapToTarget" true)
      (bind _returnvalue_2 (`KismetMaterialLibrary.CreateDynamicMaterialInstance` "/Game/Rafael/Mesh/demon-horns/source/M_DemonHorn.M_DemonHorn"))
      (`PrimitiveComponent.SetMaterial` _skel_demonhorn 0 _returnvalue_2))))

(event `Key|P`
  (params (Key :type "Key Structure")))

(event `SpawnLightBulb`)

(event `SpawnBubble`
  (params (Activate :type Boolean))
  (bind _niagara_soapbubble (`self.Niagara_SoapBubble`))
  ;[0.08854 0.08854 0.08854] Spawn Soap Bubble FX
  (if (not Activate)
    (`ActorComponent.Activate` _niagara_soapbubble false)
    (else
      (`ActorComponent.Deactivate` _niagara_soapbubble))))

(event `DemonHornApparition`
  (params (`Expression Value` :type Boolean))
  ;[0.08854 0.08854 0.08854] Change MetaHuman's Skin Color
  (bind _asmaterial_instance_dynamic (cast `MaterialInstanceDynamic` (`PrimitiveComponent.GetMaterial` (`self.Skel_DemonHorn`) 0)))
  (if (not `Expression Value`)
    (bind (_direction _erosion _hot) (`Timeline|Timeline_DemonSummoning` :!label _label)
      (:`Update`
        (`MaterialInstanceDynamic.SetScalarParameterValue` _asmaterial_instance_dynamic "Erosion" _erosion)
        (`MaterialInstanceDynamic.SetScalarParameterValue` _asmaterial_instance_dynamic "Hot" _hot)))
    (else
      (goto _label :!via `Reverse`))))

(event `ChangeHeadScale`
  (params (`Expression Value` :type Boolean) (Duration :type "Float (double-precision)"))
  ;[0.08854 0.08854 0.08854] Scale MetaHuman's Face
  (`TimelineComponent.SetPlayRate` (`self.ScaleHeadTimeline`) Duration)
  (if (not `Expression Value`)
    (bind (_direction _value) (`Timeline|ScaleHeadTimeline` :!label _label_2))
    (else
      (goto _label_2 :!via `Reverse`))))

(fn `UserConstructionScript`)