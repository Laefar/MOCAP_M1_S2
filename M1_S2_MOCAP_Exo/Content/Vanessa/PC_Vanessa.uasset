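; PC_Vanessa, apparently a player controller, triggers animated on-screen widget effects from key presses, named for anger, surprise, puffing and mouth.
; Z, A, E and R each create their matching widget, store it in a variable, add it to the viewport and play its animation.
; Every press spawns a new widget, and nothing here removes earlier ones.
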(event `Key|Z`
  (params (Key :type "Key Structure"))
  (bind _colore_var (`self.Colore_var`))
  (:`Pressed`
    (bind _returnvalue (`|CreateWidget` "/Game/Vanessa/W_colere.W_colere_C"))
    (bind _output_get (set `self.Colore_var` _returnvalue))
    (`UserWidget.AddToViewport` _output_get 0)
    (`UserWidget.PlayAnimation` _colore_var (`/Game/Vanessa/W_colere.Pentacle_anime` _colore_var) 0.0 1 "Forward" 1.0 false)))

(event `Key|A`
  (params (Key :type "Key Structure"))
  (bind _surpise_var (`self.Surpise_var`))
  (:`Pressed`
    (bind _returnvalue (`|CreateWidget` "/Game/Vanessa/W_surprise.W_surprise_C"))
    (bind _output_get (set `self.Surpise_var` _returnvalue))
    (`UserWidget.AddToViewport` _output_get 0)
    (`UserWidget.PlayAnimation` _surpise_var (`/Game/Vanessa/W_surprise.Surprise_anime` _surpise_var) 0.0 1 "Forward" 1.0 false)))

(event `Key|E`
  (params (Key :type "Key Structure"))
  (bind _gonfle_var (`self.Gonfle_var`))
  (:`Pressed`
    (bind _returnvalue (`|CreateWidget` "/Game/Vanessa/W_gonfle.W_gonfle_C"))
    (bind _output_get (set `self.Gonfle_var` _returnvalue))
    (`UserWidget.AddToViewport` _output_get 0)
    (`UserWidget.PlayAnimation` _gonfle_var (`/Game/Vanessa/W_gonfle.Gonfle_anime` _gonfle_var) 0.0 1 "Forward" 1.0 false)))

(event `Key|R`
  (params (Key :type "Key Structure"))
  (bind _bouche_var (`self.Bouche_var`))
  (:`Pressed`
    (bind _returnvalue (`|CreateWidget` "/Game/Vanessa/W_bouche.W_bouche_C"))
    (bind _output_get (set `self.Bouche_var` _returnvalue))
    (`UserWidget.AddToViewport` _output_get 0)
    (`UserWidget.PlayAnimation` _bouche_var (`/Game/Vanessa/W_bouche.Bouche_anime` _bouche_var) 0.0 1 "Forward" 1.0 false)))

(fn `UserConstructionScript`)